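; Ranged enemy character that carries a pistol and shoots as its attack.
; On BeginPlay it spawns a pistol pickup and attaches it to the mesh's hand socket, Pistol_Socket.
; Attack plays a shotgun sound, fires through BPCDamage, reduces BPCAmmo and signals attack end; the ammo check is disconnected.
; It also maps movement states to walk speeds and reports fixed attack and defend ranges.
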(event `self.ReceiveBeginPlay`
  (`self.EquipWeapon`))

(event `/Game/Enemies/AI/BPI_EnemyAI.EquipWeapon`
  (bind _returnvalue (`|SpawnActorFromClass` "/Game/_Project/Props/PickupSprites/BP_Pistol_Pickup.BP_Pistol_Pickup_C" (`KismetMathLibrary.MakeTransform` (0.0 0.0 0.0)) "Undefined" "MultiplyWithRoot" null null))
  (`self.K2_AttachToComponent` _returnvalue (`self.Mesh`) "Pistol_Socket" "KeepRelative" "KeepRelative" "KeepRelative" true))

(event `/Game/Enemies/AI/BPI_EnemyAI.Attack`
  (`GameplayStatics.PlaySoundAtLocation` "/Game/MilitaryWeapSilver/Sound/Shotgun/Wavs/ShotgunA_Fire01.ShotgunA_Fire01" (0.0 0.0 0.0) (struct) 1.0 1.0 0.0 null null null null)
  (`/Game/_Project/Components/BPC_Shooting.Shooting Handler` (`self.BPC_Damage`))
  (`KismetSystemLibrary.PrintText` "EnemyShoot")
  (`/Game/_Project/Components/BPC_Ammo.Reduce Ammo` (`self.BPC_Ammo`))
  (`self.OnAttackEnd`))

(fn `GetIdealRange`
  (returns (AttackRadius :type "Float (double-precision)") (DefendRadius :type "Float (double-precision)"))
  (return 600.0 600.0))

(fn `SetMovementSpeed`
  (params (Speed :type "/Game/Enemies/AI/Enums/E_MoveSpeed Enum" :default "NewEnumerator0"))
  (returns (SpeedValue :type "Float (double-precision)"))
  (bind _output_get (set `CharacterMovementComponent.MaxWalkSpeed` (select `/Game/Enemies/AI/Enums/E_MoveSpeed` Speed :`NewEnumerator1` 200.0 :`NewEnumerator2` 300.0 :`NewEnumerator3` 500.0 :!type "Float (single-precision)") (`self.CharacterMovement`)))
  (return _output_get))

(fn `UserConstructionScript`
  (`parent.UserConstructionScript`))