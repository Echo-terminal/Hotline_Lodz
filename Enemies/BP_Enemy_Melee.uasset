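; BP_Enemy_Melee is a melee enemy Blueprint that arms itself with a knife when play begins.
; EquipWeapon spawns a BP_Knife_Pickup and snaps it to the Knife_Socket on the enemy's mesh.
; Disconnected shooting logic with ammo checks, shotgun sound and damage component calls remains in the graph but never runs, so no attack behavior is active here.
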(event `self.ReceiveBeginPlay`
  (`self.EquipWeapon`))

(event `/Game/Enemies/AI/BPI_EnemyAI.EquipWeapon`
  (bind _returnvalue (`|SpawnActorFromClass` "/Game/_Project/Props/PickupSprites/BP_Knife_Pickup.BP_Knife_Pickup_C" (`self.GetTransform`) "Undefined" "MultiplyWithRoot" null null))
  (`self.K2_AttachToComponent` _returnvalue (`self.Mesh`) "Knife_Socket" "SnapToTarget" "SnapToTarget" "SnapToTarget" true))

(fn `UserConstructionScript`
  (`parent.UserConstructionScript`))