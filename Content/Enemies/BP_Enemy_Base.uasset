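; Base enemy character that takes damage, dies, and exposes patrol, range and movement speed functions.
; Incoming damage goes to BPCHealth, and a zero result plays the death animation and disables movement.
; Getters return the patrol route and fixed attack and defend radii, while a setter maps a speed state to max walk speed.
; The generically named NewFunction returns three random offsets within the current weapon's spread.
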(event `self.ReceiveAnyDamage`
  (params (Damage :type "Float (single-precision)") (DamageType :type "DamageType Object Reference") (InstigatedBy :type "Controller Object Reference") (DamageCauser :type "Actor Object Reference"))
  (bind _new_health (`/Game/_Project/Components/BPC_Health.Health Handler` (`self.BPC_Health`) Damage))
  (if (== _new_health 0.0)
    (`SkeletalMeshComponent.PlayAnimation` (`self.Mesh`) "/Game/_Project/Props/DeadEnemyAnim.DeadEnemyAnim" false)
    (`CharacterMovementComponent.DisableMovement` (`self.CharacterMovement`))))

(fn `GetIdealRange`
  (returns (AttackRadius :type "Float (double-precision)") (DefendRadius :type "Float (double-precision)"))
  (return 100.0 200.0))

(fn `GetPatrolRoute`
  (returns (PatrolRoute :type "/Game/Enemies/AI/BP_PatrolRoute Object Reference"))
  (return (`self.PatrolRoute`)))

(fn `NewFunction`
  (returns (ReturnValue :type "Float (double-precision)") (ReturnValue2 :type "Float (double-precision)") (ReturnValue3 :type "Float (double-precision)"))
  (bind _spread (`/Game/_Project/Props/Weapons/BP_Weapon_Parent.Spread` (`self.Current Weapon`)))
  (bind _spread_2 (`/Game/_Project/Props/Weapons/BP_Weapon_Parent.Spread` (`self.Current Weapon`)))
  (bind _spread_3 (`/Game/_Project/Props/Weapons/BP_Weapon_Parent.Spread` (`self.Current Weapon`)))
  (return (`KismetMathLibrary.RandomFloatInRange` (* _spread_3 -1.0) _spread_3) (`KismetMathLibrary.RandomFloatInRange` (* _spread -1.0) _spread) (`KismetMathLibrary.RandomFloatInRange` (* _spread_2 -1.0) _spread_2)))

(fn `SetMovementSpeed`
  (params (Speed :type "/Game/Enemies/AI/Enums/E_MoveSpeed Enum" :default "NewEnumerator0"))
  (returns (SpeedValue :type "Float (double-precision)"))
  (bind _output_get (set `CharacterMovementComponent.MaxWalkSpeed` (select `/Game/Enemies/AI/Enums/E_MoveSpeed` Speed :`NewEnumerator1` 100.0 :`NewEnumerator2` 300.0 :`NewEnumerator3` 500.0 :!type "Float (single-precision)") (`self.CharacterMovement`)))
  (return _output_get))

(fn `UserConstructionScript`)