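; BPC_Shooting is an actor component that performs hitscan weapon fire for the owning BP_ThirdPersonCharacter.
; ShootingHandler traces from the follow camera using the current weapon's range and random spread, firing seven pellets for weapon type 2 and one otherwise.
; Each trace draws debug lines, applies weapon damage to the hit actor and plays the hit cue in 2D without checking for a hit.
; The event graph's own ShootingHandler call is unconnected.
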(fn `Shooting Handler`
  (bind _asbp_third_person_character (cast `/Game/ThirdPerson/Blueprints/BP_ThirdPersonCharacter` (`self.GetOwner`)))
  (bind _current_weapon (`/Game/ThirdPerson/Blueprints/BP_ThirdPersonCharacter.Current Weapon` _asbp_third_person_character))
  (`/Engine/EditorBlueprintResources/StandardMacros.IsValid` _current_weapon
    (:`Is Valid`
      (if (== (`/Game/_Project/Props/Weapons/BP_Weapon_Parent.WeaponType` _current_weapon) 2)
        (for _ (range 1 8)
          (bind _followcamera (`/Game/ThirdPerson/Blueprints/BP_ThirdPersonCharacter.FollowCamera` _asbp_third_person_character))
          (bind _returnvalue (`SceneComponent.K2_GetComponentLocation` _followcamera))
          (bind _spread (`/Game/_Project/Props/Weapons/BP_Weapon_Parent.Spread` _current_weapon))
          (bind _outhit (`KismetSystemLibrary.LineTraceSingle` :`Start` _returnvalue :`End` (+ (* (`/Game/_Project/Props/Weapons/BP_Weapon_Parent.Range` _current_weapon) (`KismetMathLibrary.GetForwardVector` (`SceneComponent.K2_GetComponentRotation` _followcamera))) _returnvalue (`KismetMathLibrary.MakeVector` (`KismetMathLibrary.RandomFloatInRange` (* _spread -1.0) _spread) (`KismetMathLibrary.RandomFloatInRange` (* _spread -1.0) _spread) (`KismetMathLibrary.RandomFloatInRange` (* _spread -1.0) _spread))) :`TraceChannel` "TraceTypeQuery1" :`DrawDebugType` "ForDuration" :!label _label))
          (`GameplayStatics.ApplyDamage` (`.HitActor` (`GameplayStatics.BreakHitResult` _outhit)) (`/Game/_Project/Props/Weapons/BP_Weapon_Parent.Damage` _current_weapon))
          (bind _hitcue (`/Game/_Project/Props/Weapons/BP_Weapon_Parent.HitCue` _current_weapon)
            (:`then`
              (`GameplayStatics.SpawnSound2D` _hitcue 1.0 1.0 0.0 null))
            (:`else`)))
        (else
          (goto _label))))))