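; BPC_Ammo is a component that tracks ammo use for the current weapon of its owning BP_ThirdPersonCharacter.
; ReduceAmmo casts the owner to that character and subtracts one from CurrentWeapon's Ammo, with no lower limit.
; CheckAmmo returns whether that Ammo is above zero; its IsValid branch on the weapon does not alter the result.
; The count lives on the weapon, so the component holds no ammo state itself.
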(fn `Check Ammo`
  (returns (`Has Ammo` :type Boolean))
  (bind _asbp_third_person_character (cast `/Game/ThirdPerson/Blueprints/BP_ThirdPersonCharacter` (`self.GetOwner`)))
  (bind _current_weapon (`/Game/ThirdPerson/Blueprints/BP_ThirdPersonCharacter.Current Weapon` _asbp_third_person_character)
    (:`then`
      _)
    (:`else`
      _))
  (return (> (`/Game/_Project/Props/Weapons/BP_Weapon_Parent.Ammo` _current_weapon) 0)))

(fn `Reduce Ammo`
  (bind _asbp_third_person_character (cast `/Game/ThirdPerson/Blueprints/BP_ThirdPersonCharacter` (`self.GetOwner`)))
  (bind _current_weapon (`/Game/ThirdPerson/Blueprints/BP_ThirdPersonCharacter.Current Weapon` _asbp_third_person_character))
  (set `/Game/_Project/Props/Weapons/BP_Weapon_Parent.Ammo` (- (`/Game/_Project/Props/Weapons/BP_Weapon_Parent.Ammo` _current_weapon) 1) _current_weapon))